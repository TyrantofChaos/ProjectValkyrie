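; BP_DialogueComponent is a dialogue component that shows data-table-driven conversation lines in an on-screen widget, one per Interact event.
; The first Interact creates the widget with the speaker name and line, and later ones update its text.
; Each row supplies the next row name, data table and end flag, chaining lines across tables.
; Once the end flag is set, the next Interact removes the widget and clears the flag.
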(event `/Game/Dialogue/BP_Interact.Interact`
  (params (PlayerRef :type "/Game/ThirdPerson/Blueprints/BP_ThirdPersonCharacter Object Reference"))
  (if (`self.EndDialogue`)
    (`Widget.RemoveFromParent` (`.DialogueWidget` (`self.DialogueWidget`)))
    (set `self.EndDialogue` false)
    (set `self.DialogueWidget` null)
    (else
      (`/Engine/EditorBlueprintResources/StandardMacros.IsValid` (`.DialogueWidget` (`self.DialogueWidget`))
        (:`Is Valid`
          (bind _returnvalue (`|GetDataTableRow` (`self.Data Table`) (`self.Row Name`))
            (:`then`
              (bind (_dialogue _row _datatable _enddialogue) (break `/Game/Dialogue/Dialogue_Structure` _returnvalue))
              (`self.Update Dialogue` (`.DialogueWidget` (`self.DialogueWidget`)) _dialogue)
              (set `self.Row Name` _row)
              (set `self.Data Table` _datatable)
              (set `self.EndDialogue` _enddialogue))))
        (:`Is Not Valid`
          (bind _returnvalue_2 (`|GetDataTableRow` (`self.Data Table`) (`self.Row Name`))
            (:`then`
              (bind (_dialogue_2 _row_2 _datatable_2 _enddialogue_2) (break `/Game/Dialogue/Dialogue_Structure` _returnvalue_2))
              (bind _returnvalue_3 (`|CreateWidget` null null (`KismetTextLibrary.Conv_NameToText` (`self.Name`)) _dialogue_2))
              (bind (_output_get _output_get_2) (set `self.DialogueWidget` null _returnvalue_3))
              (`UserWidget.AddToViewport` _output_get_2 0)
              (set `self.Row Name` _row_2)
              (set `self.Data Table` _datatable_2)
              (set `self.EndDialogue` _enddialogue_2))))))))